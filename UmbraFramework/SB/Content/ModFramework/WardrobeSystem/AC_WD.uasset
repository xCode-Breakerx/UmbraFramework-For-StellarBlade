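; Actor component that bootstraps and fronts a modded wardrobe system on its owning character.
; InitWardrobe spawns a WardrobeTest manager actor with the mod body and the owner's "Body"-tagged skeletal mesh, and lets the owner tick while paused.
; It also disables Slate global invalidation by console command to fix unresponsive UI widgets.
; Outfit registration, default equip and skin refresh calls forward to that manager; TryLoadSaveForOutfit is a stub returning false.
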(event `/Game/ModFramework/Interface/BPI_Wardrobe.InitWardrobe`
  (params (ModBody :type "SkeletalMeshComponent Object Reference"))
  (bind _returnvalue (`self.GetOwner`))
  ;[0 0 0] ~Wardrobe interface
  (bind _returnvalue_2 (`|SpawnActorFromClass` "/Game/ModFramework/WardrobeSystem/WardrobeTest.WardrobeTest_C" (`Actor.GetTransform` _returnvalue) "AlwaysSpawn" "OverrideRootScale" _returnvalue ModBody (`|GetArrayItem` (`Actor.GetComponentsByTag` _returnvalue "/Script/Engine.SkeletalMeshComponent" "Body")) (`Actor.Instigator` _returnvalue)))
  (set `self.WardrobeManager` _returnvalue_2)
  (`Actor.SetTickableWhenPaused` (`self.GetOwner`) true)
  ;;[0 0 0] Fixes the UI responsiveness
  ;; For some reason SB has this enabled making the UI very unresponsive with vanilla widgets such as sliders
  (`KismetSystemLibrary.ExecuteConsoleCommand` "Slate.EnableGlobalInvalidation 0" (`GameplayStatics.GetPlayerController` 0)))

(event `/Game/ModFramework/Interface/BPI_Wardrobe.RegisterOutfit`
  (params (Outfit :type "/Game/ModFramework/ModConfig/Outfit/PDA_ModOutfitConfig Soft Object Reference"))
  ;[0 0 0] ~Wardrobe interface
  (bind _wardrobemanager (`self.WardrobeManager`)
    (:`then`
      (message `/Game/ModFramework/Interface/BPI_Wardrobe.RegisterOutfit` _wardrobemanager Outfit))
    (:`else`)))

(event `/Game/ModFramework/Interface/BPI_Wardrobe.EquipDefault`
  ;[0 0 0] ~Wardrobe interface
  (bind _wardrobemanager (`self.WardrobeManager`)
    (:`then`
      (message `/Game/ModFramework/Interface/BPI_Wardrobe.EquipDefault` _wardrobemanager))
    (:`else`)))

(event `/Game/ModFramework/Interface/BPI_Wardrobe.RefreshSkin`
  ;[0 0 0] ~Wardrobe interface
  (bind _wardrobemanager (`self.WardrobeManager`)
    (:`then`
      (message `/Game/ModFramework/Interface/BPI_Wardrobe.RefreshSkin` _wardrobemanager))
    (:`else`)))

(fn `TryLoadSaveForOutfit`
  (params (OutfitConfig :type "/Game/ModFramework/ModConfig/Outfit/FBP_Outfit Structure") (ModIndex :type Integer))
  (returns (OutOutfit :type "/Game/ModFramework/ModConfig/Outfit/FBP_Outfit Structure") (Accessories :type "/Game/ModFramework/ModConfig/Accessories/FBP_OutfitAccessoryConfig Structure") (ValidAccessories :type Boolean))
  (return (struct) (struct) false))